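; BP_VerifyCollision is a test actor that shows which collision events its Cube receives by changing the cube's color.
; The construction script applies collision-enabled and per-channel response settings from variables to the Cube.
; BeginPlay creates a dynamic material instance from M_ChangeColor_Inst.
; Hit, begin-overlap and end-overlap events each pass their own color to ChangeColor, which sets the material's Color parameter.
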(event OnComponentHit(Cube)
  (params (HitComponent :type Primitive%20Component%20Object%20Reference) (OtherActor :type Actor%20Object%20Reference) (OtherComp :type Primitive%20Component%20Object%20Reference) (NormalImpulse :type Vector :default "0, 0, 0") (Hit :type Hit%20Result%20Structure%20%28by%20ref%29))
  (CallFunction|ChangeColor (Variables|Default|GetColorHit)))

(event OnComponentBeginOverlap(Cube)
  (params (OverlappedComponent :type Primitive%20Component%20Object%20Reference) (OtherActor :type Actor%20Object%20Reference) (OtherComp :type Primitive%20Component%20Object%20Reference) (OtherBodyIndex :type Integer) (bFromSweep :type Boolean) (SweepResult :type Hit%20Result%20Structure%20%28by%20ref%29))
  (CallFunction|ChangeColor (Variables|Default|GetColorBeginOverlap)))

(event OnComponentEndOverlap(Cube)
  (params (OverlappedComponent :type Primitive%20Component%20Object%20Reference) (OtherActor :type Actor%20Object%20Reference) (OtherComp :type Primitive%20Component%20Object%20Reference) (OtherBodyIndex :type Integer))
  (CallFunction|ChangeColor (Variables|Default|GetColorEndOverlap)))

(event EventBeginPlay
  (bind _returnvalue (Rendering|Material|CreateDynamicMaterialInstance (Variables|Default|GetCube) 0 "/Game/Blueprints/M_ChangeColor_Inst.M_ChangeColor_Inst" :!class /Script/Engine.PrimitiveComponent))
  (Variables|Default|SetMaterialInst _returnvalue))

(event Collision|EventActorBeginOverlap
  (params (OtherActor :type Actor%20Object%20Reference)))

(event EventTick
  (params (DeltaSeconds :type Float%20%28single-precision%29)))

(fn ConstructionScript
  (Collision|SetCollisionEnabled (Variables|Default|GetCube) (Variables|Default|GetCollisionEnable))
  (Collision|SetCollisionResponsetoChannel (Variables|Default|GetCube) (Variables|Default|GetCollisionChannel) (Variables|Default|GetCollisionResponse)))

(fn ChangeColor
  (params (Color :type Linear%20Color%20Structure))
  (Rendering|Material|SetVectorParameterValue (Variables|Default|GetMaterialInst) "Color" Color :!class /Script/Engine.MaterialInstanceDynamic)
  (return true))